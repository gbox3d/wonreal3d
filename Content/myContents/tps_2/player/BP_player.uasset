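; Player character Blueprint with movement, a montage-driven melee attack and ragdoll on damage.
; Enhanced Input feeds movement and attacks to the BPCPlayerControlLib and BPCSimpleAttack components.
; StartAttackTrace loops a timer that sphere-traces between two right-hand points, applying damage and stopping on the first hit.
; Any damage received immediately ragdolls the mesh, launches it along the damage causer's forward vector and disables capsule collision.
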(event Custom|AttackTrace
  (bind (_outhit _returnvalue) (Collision|SphereTraceByChannel (Transformation|GetWorldLocation (Variables|Default|GetrHand)) (Transformation|GetWorldLocation (Variables|Default|Getrhand_end)) 2e+01 "TraceTypeQuery1" false 0 "ForDuration"))
  (if _returnvalue
    (Game|Damage|ApplyDamage (.HitActor (Collision|BreakHitResult _outhit)) 1e+01 0 self)
    (CallFunction|StopAttackTrace)))

(event Input|EnhancedActionEvents|EnhancedInputActionIA_Move
  (params (ActionValue :type Vector%202D%20Structure) (ElapsedSeconds :type Float%20%28double-precision%29) (TriggeredSeconds :type Float%20%28double-precision%29) (InputAction :type Input%20Action%20Object%20Reference :default "/Game/Input/Actions/IA_Move.IA_Move"))
  (Default|Move (Variables|Default|GetBPC_player_control_lib) self (.x ActionValue) (.y ActionValue)))

(event Input|EnhancedActionEvents|EnhancedInputActionIA_attack
  (params (ActionValue :type Boolean) (ElapsedSeconds :type Float%20%28double-precision%29) (TriggeredSeconds :type Float%20%28double-precision%29) (InputAction :type Input%20Action%20Object%20Reference :default "/Game/myContents/input/IA_attack.IA_attack"))
  (Default|StartAttack (Variables|Default|GetBPC_SimpleAttack) (Variables|Character|GetMesh) "/Game/myContents/tps_2/MM_Attack_01_Montage.MM_Attack_01_Montage"))

(event EventStopAttackTrace
  (Utilities|Time|ClearandInvalidateTimerbyHandle (Variables|Default|GettraceTimerHandler)))

(event Game|Damage|EventAnyDamage
  (params (Damage :type Float%20%28single-precision%29) (DamageType :type Damage%20Type%20Object%20Reference) (InstigatedBy :type Controller%20Object%20Reference) (DamageCauser :type Actor%20Object%20Reference))
  (bind _mesh (Variables|Character|GetMesh))
  (Physics|SetSimulatePhysics _mesh true)
  (Collision|SetCollisionProfileName _mesh "Ragdoll" true :!class /Script/Engine.PrimitiveComponent)
  (Physics|AddImpulse _mesh (* (Transformation|GetActorForwardVector DamageCauser) 1e+04) "None" true)
  (Collision|SetCollisionEnabled (Variables|Collision|GetCapsuleComponent) "NoCollision"))

(event EventControllerChanged
  (params (OldController :type Controller%20Object%20Reference) (NewController :type Controller%20Object%20Reference))
  (bind _asplayer_controller (Utilities|Casting|CastToPlayerController NewController))
  (bind _output_get (Variables|Default|SetPlayer%20Controller _asplayer_controller))
  (Input|AddMappingContext (PlayerController|LocalPlayerSubsystems|GetEnhancedInputLocalPlayerSubsystem _output_get) "/Game/myContents/input/IMC_Default.IMC_Default" 0 "(bIgnoreAllPressedKeysUntilRelease=True,bForceImmediately=False,bNotifyUserSettings=False)"))

(event EventStartAttackTrace
  (bind _returnvalue (Utilities|Time|SetTimerbyEvent (delegate Custom|AttackTrace) 0.01 true))
  (Variables|Default|SettraceTimerHandler _returnvalue))

(fn ConstructionScript)