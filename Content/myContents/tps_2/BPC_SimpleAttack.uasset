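; BPC_SimpleAttack is a simple attack component that plays an attack montage and can knock a hit mesh away.
; StartAttack plays the given montage on a skeletal mesh, with an IsAttacking flag that blocks repeat attacks until the montage completes.
; BlowAway prints a debug message, turns the mesh into a physics ragdoll and launches it along the passed actor's forward vector with a velocity-change impulse.
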(event Custom|StartAttack
  (params (InSkeletalMeshComponent :type Skeletal%20Mesh%20Component%20Object%20Reference) (MontageToPlay :type Anim%20Montage%20Object%20Reference))
  (if (not (Variables|Default|Getis%20attacking))
    (Variables|Default|Setis%20attacking true)
    (Animation|Montage|PlayMontage InSkeletalMeshComponent MontageToPlay
      (:OnCompleted
        (Variables|Default|Setis%20attacking false)))))

(fn BlowAway
  (params (mesh :type Primitive%20Component%20Object%20Reference) (actor :type Actor%20Object%20Reference))
  (Development|PrintString "hit")
  (Physics|SetSimulatePhysics mesh true)
  (Collision|SetCollisionProfileName mesh "Ragdoll" true :!class /Script/Engine.PrimitiveComponent)
  (Physics|AddImpulse mesh (* (Transformation|GetActorForwardVector actor) 1e+04) "None" true))