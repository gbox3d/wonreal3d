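; AI enemy character that targets the player and deals melee damage with its left hand.
; A sphere overlap passes the player to AIC_AIPlayer as the target.
; A looping timer, started and stopped by events, sphere-traces between left-hand points and applies damage on the first hit.
; Any damage ragdolls it with an impulse along the damage causer's forward vector, unpossesses it, disables capsule collision, then destroys it after a delay.
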(event OnComponentBeginOverlap(Sphere)
  (params (OverlappedComponent :type Primitive%20Component%20Object%20Reference) (OtherActor :type Actor%20Object%20Reference) (OtherComp :type Primitive%20Component%20Object%20Reference) (OtherBodyIndex :type Integer) (bFromSweep :type Boolean) (SweepResult :type Hit%20Result%20Structure%20%28by%20ref%29))
  (bind _asbp_player (Utilities|Casting|CastToBP_player OtherActor))
  (bind _asaic_aiplayer (Utilities|Casting|CastToAIC_AIPlayer (AI|GetAIController self)))
  (Default|SetTarget _asaic_aiplayer _asbp_player))

(event Custom|AttackTrace
  (bind (_outhit _returnvalue) (Collision|SphereTraceByChannel (Transformation|GetWorldLocation (Variables|Default|GetlHandBegin)) (Transformation|GetWorldLocation (Variables|Default|GetlHandEnd)) 2e+01 "TraceTypeQuery2" false 0 "ForDuration"))
  (if _returnvalue
    (Game|Damage|ApplyDamage (.HitActor (Collision|BreakHitResult _outhit)) 1e+01 0 self)
    (CallFunction|StopAttackTrace)))

(event EventStartAttackTrace
  (bind _returnvalue (Utilities|Time|SetTimerbyEvent (delegate Custom|AttackTrace) 0.01 true))
  (Variables|Default|Setattack%20trace%20timer%20handler _returnvalue))

(event EventStopAttackTrace
  (Utilities|Time|ClearandInvalidateTimerbyHandle (Variables|Default|Getattack%20trace%20timer%20handler)))

(event Game|Damage|EventAnyDamage
  (params (Damage :type Float%20%28single-precision%29) (DamageType :type Damage%20Type%20Object%20Reference) (InstigatedBy :type Controller%20Object%20Reference) (DamageCauser :type Actor%20Object%20Reference))
  (Physics|SetSimulatePhysics (Variables|Character|GetMesh) true)
  (Collision|SetCollisionProfileName (Variables|Character|GetMesh) "Ragdoll" true :!class /Script/Engine.PrimitiveComponent)
  (Physics|AddImpulse (Variables|Character|GetMesh) (* (Transformation|GetActorForwardVector DamageCauser) 5e+03) "None" true)
  (Pawn|UnPossess (Pawn|GetController))
  (Collision|SetCollisionEnabled (Variables|Collision|GetCapsuleComponent) "NoCollision")
  (Utilities|FlowControl|Delay 1e+01)
  (Actor|DestroyActor))

(fn ConstructionScript)