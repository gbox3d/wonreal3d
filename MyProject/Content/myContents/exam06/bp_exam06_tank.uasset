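; Tank actor Blueprint for an exam exercise that turns and drives itself every Tick from the NTurn and Forward variables.
; A Sequence first applies a local yaw rotation scaled by NTurn, then a local offset along the X axis scaled by Forward.
; Both steps scale by delta time for frame-rate-independent motion, and the move does not sweep for collision.
; Nothing in these graphs sets either variable.
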(event EventBeginPlay)

(event Collision|EventActorBeginOverlap
  (params (OtherActor :type Actor%20Object%20Reference)))

(event EventTick
  (params (DeltaSeconds :type Float%20%28single-precision%29))
  (Utilities|FlowControl|Sequence
    (:then_0
      (Transformation|AddActorLocalRotation (Math|Rotator|MakeRotator 0.0 0.0 (* (* DeltaSeconds 45.0) (Variables|Default|GetnTurn))) false false))
    (:then_1
      (Transformation|AddActorLocalOffset (* (Math|Vector|GetForwardVector "0, 0, 0") (* (* DeltaSeconds 1e+02) (Variables|Default|Getforward))) false false))))

(fn ConstructionScript)